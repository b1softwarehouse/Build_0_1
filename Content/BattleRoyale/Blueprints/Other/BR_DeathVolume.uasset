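; Battle royale shrinking zone actor that damages the player every two seconds while outside the damage wall once the game has started.
; The safe wall marks the next zone, spawned within SpawnBox, then shrunk and re-centered inside its previous radius using square-root polar sampling, flipping centers that leave the box.
; Tick lerps the damage wall onto the safe wall over a given duration and updates the game mode's shrinking flag.
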(event OnComponentEndOverlap(DamageWall)
  (params (OverlappedComponent :type Primitive%20Component%20Object%20Reference) (OtherActor :type Actor%20Object%20Reference) (OtherComp :type Primitive%20Component%20Object%20Reference) (OtherBodyIndex :type Integer))
  ;[1 1 1] If the player is no longer overlapping with the damage wall, start damaging the player
  (bind _asbr_character (Utilities|Casting|CastToBR_Character OtherActor))
  (if (and (Variables|/Game/BattleRoyale/Blueprints/BR_Character.BR_Character_C|GetIsPlayer _asbr_character) (Variables|/Game/BattleRoyale/Blueprints/BR_GameMode.BR_GameMode_C|GetIsGameStarted (.AsBR%20Game%20Mode (Utilities|Casting|CastToBR_GameMode (Game|GetGameMode)))))
    (Variables|Default|SetCharToDamage _asbr_character)
    (bind _returnvalue (Utilities|Time|SetTimerbyEvent (delegate Custom|DamagePlayer) 2.0 true))
    (Variables|Default|SetDamTimerHandle _returnvalue)))

(event OnComponentBeginOverlap(DamageWall)
  (params (OverlappedComponent :type Primitive%20Component%20Object%20Reference) (OtherActor :type Actor%20Object%20Reference) (OtherComp :type Primitive%20Component%20Object%20Reference) (OtherBodyIndex :type Integer) (bFromSweep :type Boolean) (SweepResult :type Hit%20Result%20Structure%20%28by%20ref%29))
  ;[1 1 1] If the player is inside the damage wall (new overlap), stop damaging the player
  (bind _asbr_character (Utilities|Casting|CastToBR_Character OtherActor))
  (if (and (Variables|/Game/BattleRoyale/Blueprints/BR_Character.BR_Character_C|GetIsPlayer _asbr_character) (Variables|/Game/BattleRoyale/Blueprints/BR_GameMode.BR_GameMode_C|GetIsGameStarted (.AsBR%20Game%20Mode (Utilities|Casting|CastToBR_GameMode (Game|GetGameMode)))))
    (Utilities|Time|ClearandInvalidateTimerbyHandle (Variables|Default|GetDamTimerHandle))
    (Variables|Default|SetCharToDamage 0)))

(event Custom|DamagePlayer
  ;[1 1 1] If the player is no longer overlapping with the damage wall, start damaging the player
  (Game|Damage|ApplyDamage (Variables|Default|GetCharToDamage) (Variables|Default|GetDamage) 0 self))

(event EventBeginPlay
  ;[1 1 1] When this gets created, set the default wall values
  (CallFunction|SetDefaultValues))

(event EventMoveandShrinkDamageWall
  (params (ShrinkDuration :type Float%20%28single-precision%29))
  ;[1 1 1] Move and Shrink Damage Wall implementation - set the appropriate variables, the tick function will do the shrinking
  (Variables|Default|SetWallShrinkDuration ShrinkDuration)
  (Variables|Default|SetStartingWallTransform (Transformation|GetWorldTransform (Variables|Default|GetDamageWall)))
  (bind _output_get (Variables|Default|SetShouldShrinkWall true))
  (Variables|/Game/BattleRoyale/Blueprints/BR_GameMode.BR_GameMode_C|SetIsWallShrinking (.AsBR%20Game%20Mode (Utilities|Casting|CastToBR_GameMode (Game|GetGameMode))) _output_get))

(event EventUpdateSafeZone
  (params (XFactor :type Float%20%28single-precision%29) (YFactor :type Float%20%28single-precision%29) (ScaleFactor :type Float%20%28single-precision%29) (Damage :type Float%20%28single-precision%29))
  ;[1 1 1] Update Safe Zone implementation
  (CallFunction|UpdateMySafeZone XFactor YFactor ScaleFactor Damage))

(event EventUpdateFinalDamage
  (params (Damage :type Float%20%28single-precision%29))
  ;[1 1 1] Update the final damage number when there are no more shrinking loops
  (CallFunction|UpdateDamage Damage))

(event EventSetDefaultValues
  ;[1 1 1] Set Default Values implementation - so the walls can be reset properly
  (Variables|Default|SetDefaultSafeWall (Transformation|GetRelativeTransform (Variables|Default|GetSafeWall)))
  (Variables|Default|SetDefaultDamageWall (Transformation|GetRelativeTransform (Variables|Default|GetDamageWall))))

(event EventSpawnNewSafeZone
  (params (XFactor :type Float%20%28single-precision%29) (YFactor :type Float%20%28single-precision%29) (ScalePercent :type Float%20%28single-precision%29) (Damage :type Float%20%28single-precision%29))
  ;[1 1 1] Spawn New Safe Zone implementation
  (CallFunction|SpawnSafeZone XFactor YFactor ScalePercent Damage))

(event EventTick
  (params (DeltaSeconds :type Float%20%28single-precision%29))
  ;[1 1 1] On the tick event, if the wall should be shrinking, get the current percentage of time elapsed and how long it should take for the wall to shrink and send it to the move wall function.  If time is up, send 1 to move wall and set variables to stop shrinking
  (if (Variables|Default|GetShouldShrinkWall)
    (bind _output_get (Variables|Default|SetCurrentShrinkDuration (+ (Utilities|Time|GetWorldDeltaSeconds) (Variables|Default|GetCurrentShrinkDuration))))
    (if (> (/ _output_get (Variables|Default|GetWallShrinkDuration)) 1.0)
      (CallFunction|MoveDamageWall 1.0)
      (Variables|Default|SetShouldShrinkWall false)
      (Variables|Default|SetCurrentShrinkDuration 0.0)
      (Variables|/Game/BattleRoyale/Blueprints/BR_GameMode.BR_GameMode_C|SetIsWallShrinking (.AsBR%20Game%20Mode (Utilities|Casting|CastToBR_GameMode (Game|GetGameMode))) false)
      (else
        (CallFunction|MoveDamageWall (/ _output_get (Variables|Default|GetWallShrinkDuration)))))))

(event EventResetAlltoDefault
  ;[1 1 1] Reset All to Default implementation
  (CallFunction|ResetVariables))

(fn ConstructionScript)

(fn SpawnSafeZone
  (params (XFactor :type Float%20%28single-precision%29) (YFactor :type Float%20%28single-precision%29) (ScalePercent :type Float%20%28single-precision%29) (Damage :type Float%20%28single-precision%29))
  (bind _spawnbox (Variables|Default|GetSpawnBox))
  (bind _safewall (Variables|Default|GetSafeWall))
  (bind _returnvalue (Transformation|GetWorldScale _safewall))
  (bind _boxextent (Variables|/Script/Engine.BoxComponent|GetBoxExtent _spawnbox))
  ;[1 1 1] Spawn the safe zone with regards to the scale and x/y factors along with the spawn box
  (LocalVariables|SetLocalXFactor XFactor)
  (LocalVariables|SetLocalYFactor YFactor)
  (LocalVariables|SetLocalScalePercent ScalePercent)
  (LocalVariables|SetLocalNewDamage Damage)
  (Transformation|SetRelativeLocation (Variables|Default|GetSafeWall) (Math|Vector|MakeVector (* (LocalVariables|GetLocalXFactor) (.x _boxextent)) (* (LocalVariables|GetLocalYFactor) (.y _boxextent)) (.z (Variables|/Script/Engine.SceneComponent|GetRelativeLocation (Variables|Default|GetSafeWall)))) false false)
  (Transformation|SetWorldScale3D (Variables|Default|GetSafeWall) (Math|Vector|MakeVector (* (.x _returnvalue) (LocalVariables|GetLocalScalePercent)) (* (.y _returnvalue) (LocalVariables|GetLocalScalePercent)) (.z _returnvalue)))
  (Development|SetHiddeninGame (Variables|Default|GetDamageWall) false false)
  (Development|SetHiddeninGame (Variables|Default|GetSafeWall) false false)
  (Variables|Default|SetDamage (LocalVariables|GetLocalNewDamage)))

(fn ResetVariables
  ;[1 1 1] Reset walls back to default transform and hide them
  (Transformation|SetRelativeTransform (Variables|Default|GetSafeWall) (Variables|Default|GetDefaultSafeWall) false false)
  (Transformation|SetRelativeTransform (Variables|Default|GetDamageWall) (Variables|Default|GetDefaultDamageWall) false false)
  (Development|SetHiddeninGame (Variables|Default|GetDamageWall) true false)
  (Development|SetHiddeninGame (Variables|Default|GetSafeWall) true false)
  (Variables|Default|SetDamage 0.0))

(fn MoveDamageWall
  (params (Alpha :type Float%20%28single-precision%29))
  ;[1 1 1] Lerp from the starting wall transform to the safe wall transform (shrink into safe wall
  (Transformation|SetWorldTransform (Variables|Default|GetDamageWall) (Math|Transform|Lerp(Transform) (Variables|Default|GetStartingWallTransform) (Transformation|GetWorldTransform (Variables|Default|GetSafeWall)) Alpha) false false))

(fn UpdateMySafeZone
  (params (XFactor :type Float%20%28single-precision%29) (YFactor :type Float%20%28single-precision%29) (ScaleFactor :type Float%20%28single-precision%29) (Damage :type Float%20%28single-precision%29))
  (bind _safewall (Variables|Default|GetSafeWall))
  (bind _safewall_2 (Variables|Default|GetSafeWall))
  (bind _returnvalue (Transformation|GetWorldScale _safewall_2))
  (bind _returnvalue_2 (Transformation|GetRelativeTransform _safewall))
  (bind (_x _y) (Math|Vector|BreakVector (.location _returnvalue_2)))
  ;[1 1 1] Use incoming random factors along with math to calculate the safe zone's new center (X,Y) and scale (radius).
  (LocalVariables|SetLocalXFactor XFactor)
  (LocalVariables|SetLocalYFactor YFactor)
  (LocalVariables|SetLocalNewScaleFactor ScaleFactor)
  (LocalVariables|SetLocalNewDamage Damage)
  (LocalVariables|SetLocalOldScale (.X (Math|Vector|BreakVector (Transformation|GetWorldScale _safewall))))
  (LocalVariables|SetLocalNonScaledRadius (.X (Math|Vector|BreakVector (.Max (Components|StaticMesh|GetLocalBounds _safewall)))))
  (LocalVariables|SetLocalOldXCenter _x)
  (LocalVariables|SetLocalOldYCenter _y)
  (LocalVariables|SetLocalOldRadius (* (LocalVariables|GetLocalOldScale) (LocalVariables|GetLocalNonScaledRadius)))
  (LocalVariables|SetLocalNewRadius (* (LocalVariables|GetLocalNonScaledRadius) (* (LocalVariables|GetLocalOldScale) (LocalVariables|GetLocalNewScaleFactor))))
  (bind _output_get (LocalVariables|SetLocalRStar (- (LocalVariables|GetLocalOldRadius) (LocalVariables|GetLocalNewRadius))))
  (LocalVariables|SetLocalRPrime (* (Math|Float|Absolute(Float) (LocalVariables|GetLocalXFactor)) (Math|Float|Square _output_get)))
  (LocalVariables|SetLocalSigma (* (* (Math|Trig|GetPI) 2.0) (Math|Float|Absolute(Float) (LocalVariables|GetLocalYFactor))))
  (LocalVariables|SetLocalNewX (+ (* (Math|Trig|Cos(Radians) (LocalVariables|GetLocalSigma)) (Math|Float|Sqrt (LocalVariables|GetLocalRPrime))) (LocalVariables|GetLocalOldXCenter)))
  (LocalVariables|SetLocalNewY (+ (* (Math|Float|Sqrt (LocalVariables|GetLocalRPrime)) (Math|Trig|Sin(Radians) (LocalVariables|GetLocalSigma))) (LocalVariables|GetLocalOldYCenter)))
  (Utilities|FlowControl|Sequence
    (:then_0
      ;[1 1 1] Check to see if the new X center is outside the play area, if so, change the angle so it will be inside the circle (mirror over Y axis)
      (if (> (Math|Float|Absolute(Float) (LocalVariables|GetLocalNewX)) (.x (Variables|/Script/Engine.BoxComponent|GetBoxExtent (Variables|Default|GetSpawnBox))))
        (if (>= (LocalVariables|GetLocalSigma) (Math|Trig|GetPI))
          (LocalVariables|SetLocalNewX (+ (* (Math|Trig|Cos(Radians) (- (LocalVariables|GetLocalSigma) (Math|Trig|GetPI))) (Math|Float|Sqrt (LocalVariables|GetLocalRPrime))) (LocalVariables|GetLocalOldXCenter)))
          (else
            (LocalVariables|SetLocalNewX (+ (* (Math|Trig|Cos(Radians) (+ (LocalVariables|GetLocalSigma) (Math|Trig|GetPI))) (Math|Float|Sqrt (LocalVariables|GetLocalRPrime))) (LocalVariables|GetLocalOldXCenter)))))))
    (:then_1
      ;[1 1 1] Check to see if the new Y center is outside the playarea, if so, change the angle so it will be inside the circle, mirror over X axis
      (if (> (Math|Float|Absolute(Float) (LocalVariables|GetLocalNewY)) (.y (Variables|/Script/Engine.BoxComponent|GetBoxExtent (Variables|Default|GetSpawnBox))))
        (if (>= (LocalVariables|GetLocalSigma) (Math|Trig|GetPI))
          (LocalVariables|SetLocalNewY (+ (* (Math|Trig|Sin(Radians) (- (LocalVariables|GetLocalSigma) (Math|Trig|GetPI))) (Math|Float|Sqrt (LocalVariables|GetLocalRPrime))) (LocalVariables|GetLocalOldYCenter)))
          (else
            (LocalVariables|SetLocalNewY (+ (* (Math|Trig|Sin(Radians) (+ (LocalVariables|GetLocalSigma) (Math|Trig|GetPI))) (Math|Float|Sqrt (LocalVariables|GetLocalRPrime))) (LocalVariables|GetLocalOldYCenter)))))))
    (:then_2
      ;[1 1 1] Set the location and scale of the safe zone
      (Transformation|SetRelativeLocation (Variables|Default|GetSafeWall) (Math|Vector|MakeVector (LocalVariables|GetLocalNewX) (LocalVariables|GetLocalNewY) (.z (.location (Transformation|GetRelativeTransform (Variables|Default|GetSafeWall))))) false false)
      (Transformation|SetWorldScale3D (Variables|Default|GetSafeWall) (Math|Vector|MakeVector (* (.x _returnvalue) (LocalVariables|GetLocalNewScaleFactor)) (* (.y _returnvalue) (LocalVariables|GetLocalNewScaleFactor)) (.z _returnvalue)))
      (Variables|Default|SetDamage (LocalVariables|GetLocalNewDamage)))))

(fn UpdateDamage
  (params (Damage :type Float%20%28single-precision%29))
  ;[1 1 1] Updating Damage to deal to players outside play area
  (Variables|Default|SetDamage Damage))