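; Menu game mode for the non-streaming Battle Royale game, handling GameSparks connection, sign-in and matchmaking.
; On BeginPlay it binds GameInstance dispatchers to its GameSparks handlers and marks the instance as non-streaming.
; Sign-in tries registration first, falling back to authentication when that fails for an existing player.
; GameSparks delegates report results to the GameInstance, storing the RT session and participants when a match is found.
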(event OnGameSparksAvailableDelegate(GameSparks)
  (params (available :type Boolean))
  (bind _gameinstance (Variables|Default|GetGameInstance))
  ;[1 1 1] GSAvailableDelegate - set GameInstance variable and call function
  (Variables|/Game/BattleRoyale/Blueprints/BR_GameInstance.BR_GameInstance_C|SetbGSAvailable _gameinstance available)
  (Default|GSAvailable _gameinstance))

(event OnMatchFoundMessage(GSMessageListeners)
  (params (MatchFoundMessage :type GS%20Match%20Found%20Message%20Structure))
  (bind (_hasaccesstoken _accesstoken _hashost _host _hasmatchdata _matchdata _hasmatchgroup _matchgroup _hasmatchid _matchid _hasmatchshortcode _matchshortcode _hasmessageid _messageid _hasnotification _notification _hasparticipants _participants _hasport _port) (Utilities|Struct|BreakGSMatchFoundMessage MatchFoundMessage))
  (bind _gameinstance (Variables|Default|GetGameInstance))
  ;[1 1 1] GS - Match Found Delegate - set GameInstance variables and call MatchFound function
  (bind _returnvalue (Class|GSRTSession|CreateRTSession _host (Utilities|String|ToString(Integer) _port) _accesstoken))
  (Variables|/Game/BattleRoyale/Blueprints/BR_GameInstance.BR_GameInstance_C|SetSession _gameinstance _returnvalue)
  (Variables|/Game/BattleRoyale/Blueprints/BR_GameInstance.BR_GameInstance_C|SetParticipants _gameinstance _participants)
  (Default|GSMatchFound _gameinstance))

(event OnMatchNotFoundMessage(GSMessageListeners)
  (params (MatchNotFoundMessage :type GS%20Match%20Not%20Found%20Message%20Structure))
  ;[1 1 1] MatchNotFound delegate - call GameInstance function
  (Default|GSMatchNotFound (Variables|Default|GetGameInstance)))

(event Custom|GSDisconnect
  ;[1 1 1] Call Disconnect on GS component
  (Class|GameSparksComponent|Disconnect (Variables|Default|GetGameSparks)))

(event Custom|GSMatchmake
  ;[1 1 1] GSMatchMake - use GameInstance variable to matchmake and set IsCurrentlyMatching
  (|SendMatchmakingRequest "" 0 0 "" (Variables|/Game/BattleRoyale/Blueprints/BR_GameInstance.BR_GameInstance_C|GetCurrentMatchShortCode (Variables|Default|GetGameInstance)) 0 1 0 false
    (:then
      (Variables|/Game/BattleRoyale/Blueprints/BR_GameInstance.BR_GameInstance_C|SetIsCurrentlyMatching (Variables|Default|GetGameInstance) true))))

(event Custom|GSAuthenticateUser
  (params (UserName :type Text) (Password :type Text))
  (bind _returnvalue (Utilities|String|ToString(Text) UserName))
  (bind _returnvalue_2 (Utilities|String|ToString(Text) Password))
  (bind _gameinstance (Variables|Default|GetGameInstance))
  ;[1 1 1] GSAuthenticateUser - authenticate and set GameInstance variables and call proper GameInstance functions
  (bind (_registrationresponse _haserrors) (|SendRegistrationRequest _returnvalue _returnvalue_2 0 _returnvalue 0 false)
    (:OnResponse
      (if _haserrors
        (if (.NewPlayer (Utilities|Struct|BreakGSRegistrationResponse _registrationresponse))
          (Default|GSAuthFailure (Variables|Default|GetGameInstance))
          (else
            (bind _haserrors_2 (|SendAuthenticationRequest _returnvalue_2 _returnvalue 0 false)
              (:OnResponse
                (if _haserrors_2
                  (Default|GSAuthFailure (Variables|Default|GetGameInstance))
                  (else
                    (Variables|/Game/BattleRoyale/Blueprints/BR_GameInstance.BR_GameInstance_C|SetDisplayName _gameinstance _returnvalue)
                    (Default|GSAuthSuccess _gameinstance)))))))
        (else
          (Variables|/Game/BattleRoyale/Blueprints/BR_GameInstance.BR_GameInstance_C|SetDisplayName (Variables|Default|GetGameInstance) _returnvalue)
          (Default|GSAuthSuccess (Variables|Default|GetGameInstance)))))))

(event Custom|BoundAuthUser
  (params (Username :type Text) (Password :type Text))
  ;[1 1 1] Begin Play - Set up all event dispatcher calls
  (CallFunction|GSAuthenticateUser Username Password))

(event Custom|BoundInitialConnect
  ;[1 1 1] Begin Play - Set up all event dispatcher calls
  (CallFunction|InitialGSConnect))

(event Custom|BoundLogout
  ;[1 1 1] Begin Play - Set up all event dispatcher calls
  (CallFunction|GSLogout))

(event Custom|BoundDisconnect
  ;[1 1 1] Begin Play - Set up all event dispatcher calls
  (CallFunction|GSDisconnect))

(event Custom|BoundMatchmake
  ;[1 1 1] Begin Play - Set up all event dispatcher calls
  (CallFunction|GSMatchmake))

(event Custom|GSCancelMatchmaking
  ;[1 1 1] GSCancelMatchmaking - call cancel matchmaking with GI variables and set IsCurrentlyMatching
  (|SendMatchmakingRequest "cancel" 0 0 "" (Variables|/Game/BattleRoyale/Blueprints/BR_GameInstance.BR_GameInstance_C|GetCurrentMatchShortCode (Variables|Default|GetGameInstance)) 0 1 0 false
    (:then
      (Variables|/Game/BattleRoyale/Blueprints/BR_GameInstance.BR_GameInstance_C|SetIsCurrentlyMatching (Variables|Default|GetGameInstance) false))))

(event Custom|BoundCancelMatching
  ;[1 1 1] Begin Play - Set up all event dispatcher calls
  (CallFunction|GSCancelMatchmaking))

(event Custom|GSLogout
  ;[1 1 1] Logout and call the Logout dispatcher to change levels
  (Class|GameSparksComponent|Logout (Variables|Default|GetGameSparks))
  (Default|CallGSLogoutDispatcher))

(event Custom|InitialGSConnect
  (bind _gameinstance (Variables|Default|GetGameInstance))
  ;[1 1 1] InitialGSConnect - use GameInstance variables to connect
  (if (Variables|/Game/BattleRoyale/Blueprints/BR_GameInstance.BR_GameInstance_C|GetbGSAvailable _gameinstance)
    (Default|GSAvailable (Variables|Default|GetGameInstance))
    (else
      (Class|GameSparksComponent|Connect (Variables|Default|GetGameSparks) (Variables|/Game/BattleRoyale/Blueprints/BR_GameInstance.BR_GameInstance_C|GetApiKey _gameinstance) (Variables|/Game/BattleRoyale/Blueprints/BR_GameInstance.BR_GameInstance_C|GetSecret _gameinstance) true false))))

(event EventBeginPlay
  ;[1 1 1] Begin Play - Set up all event dispatcher calls
  (bind _asbr_game_instance (Utilities|Casting|CastToBR_GameInstance (Game|GetGameInstance)))
  (bind _output_get (Variables|Default|SetGameInstance _asbr_game_instance))
  (EventDispatchers|BindEventtoGIShutdown _output_get (delegate Custom|BoundDisconnect))
  (EventDispatchers|BindEventtoGSLogoutDispatcher (Variables|Default|GetGameInstance) (delegate Custom|BoundLogout))
  (EventDispatchers|BindEventtoInitialGSConnectDispatcher (Variables|Default|GetGameInstance) (delegate Custom|BoundInitialConnect))
  (EventDispatchers|BindEventtoGSAuthenticateUserDispatcher (Variables|Default|GetGameInstance) (delegate Custom|BoundAuthUser))
  (EventDispatchers|BindEventtoGSMatchmakeDispatcher (Variables|Default|GetGameInstance) (delegate Custom|BoundMatchmake))
  (EventDispatchers|BindEventtoGSCancelMMDispatcher (Variables|Default|GetGameInstance) (delegate Custom|BoundCancelMatching))
  (Variables|/Game/BattleRoyale/Blueprints/BR_GameInstance.BR_GameInstance_C|SetIsStreaming (Variables|Default|GetGameInstance) false))

(event EventTick
  (params (DeltaSeconds :type Float%20%28single-precision%29)))

(fn ConstructionScript)