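; Battle royale usable pickup that gives the using character every ammo type in its AmmoBox array at once.
; OnUsed sets an InUse lock, passes each entry to the character's AddAmmo and stores the returned count back in the box.
; An emptied box is deleted through BR_GameMode; otherwise the lock is released and the remaining ammo is sent to the game mode by GUID.
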(event EventBeginPlay)

(event Collision|EventActorBeginOverlap
  (params (OtherActor :type Actor%20Object%20Reference)))

(event EventOnUsed
  (params (Character :type BR%20Character%20Object%20Reference))
  ;[1 1 1] OnUsed override to add all the types of ammo to the character
  (if (not (Variables|Default|GetInUse))
    (bind _output_get (Variables|Default|SetInUse true))
    (Default|SendUpdatePickupinUse (.AsBR%20Game%20Mode (Utilities|Casting|CastToBR_GameMode (Game|GetGameMode))) _output_get (Variables|Default|GetGUID))
    (for (_array_element _array_index) (Variables|Default|GetAmmoBox)
      (bind _ammoleftover (Default|AddAmmo Character _array_element))
      (Utilities|Array|SetArrayElem (Variables|Default|GetAmmoBox) _array_index (Utilities|Struct|MakeSTRUCT_Ammo (.WeaponType (Utilities|Struct|BreakSTRUCT_Ammo _array_element)) (.MaxInventoryCount (Utilities|Struct|BreakSTRUCT_Ammo _array_element)) _ammoleftover)))
    (Variables|Default|SetShouldDelete true)
    (for _array_element_2 (Variables|Default|GetAmmoBox)
      (if (> (.CurrentCount (Utilities|Struct|BreakSTRUCT_Ammo _array_element_2)) 0)
        (Variables|Default|SetShouldDelete false)))
    (if (Variables|Default|GetShouldDelete)
      (Default|DeletefromGroundItems (.AsBR%20Game%20Mode (Utilities|Casting|CastToBR_GameMode (Game|GetGameMode))) self)
      (else
        (Variables|Default|SetInUse false)
        (Default|SendUpdateAllAmmoPickup (.AsBR%20Game%20Mode (Utilities|Casting|CastToBR_GameMode (Game|GetGameMode))) (Variables|Default|GetGUID) (Variables|Default|GetAmmoBox))
        (Default|SendUpdatePickupinUse (.AsBR%20Game%20Mode (Utilities|Casting|CastToBR_GameMode (Game|GetGameMode))) false (Variables|Default|GetGUID))))))

(event EventTick
  (params (DeltaSeconds :type Float%20%28single-precision%29)))

(fn ConstructionScript
  (Variables|Default|SetUseText (Utilities|Text|ToText(String) (Utilities|String|MakeLiteralString "Ammo")))
  (|CallParentFunction))