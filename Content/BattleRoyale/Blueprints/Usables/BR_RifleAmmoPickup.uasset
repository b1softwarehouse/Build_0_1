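; Battle royale usable pickup that gives rifle ammo to the character who uses it and shows its count in the use prompt.
; OnUsed sets an InUse lock, sends the pickup state by GUID through BR_GameMode for multiplayer, then calls the character's AddAmmo.
; A positive return becomes the remaining count, refreshing the prompt and re-sending the unlocked state.
; Otherwise the game mode deletes it from ground items.
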(event EventBeginPlay)

(event Collision|EventActorBeginOverlap
  (params (OtherActor :type Actor%20Object%20Reference)))

(event EventTick
  (params (DeltaSeconds :type Float%20%28single-precision%29)))

(event EventOnUsed
  (params (Character :type BR%20Character%20Object%20Reference))
  ;[1 1 1] OnUsed Override to Add Rifle Ammo to Character
  (if (not (Variables|Default|GetInUse))
    (Variables|Default|SetInUse true)
    (Default|SendUpdateAmmoPickup (.AsBR%20Game%20Mode (Utilities|Casting|CastToBR_GameMode (Game|GetGameMode))) (Variables|Default|GetInUse) (Variables|Default|GetAmmoCount) (Variables|Default|GetGUID))
    (bind _ammoleftover (Default|AddAmmo Character (Utilities|Struct|MakeSTRUCT_Ammo "/Game/BattleRoyale/Blueprints/Weapons/BR_Rifle.BR_Rifle_C" 0 (Variables|Default|GetAmmoCount))))
    (if (> _ammoleftover 0)
      ;;[1 1 1] Multiplayer
      (Variables|Default|SetAmmoCount _ammoleftover)
      (Variables|Default|SetUseText (Utilities|Text|ToText(String) (Utilities|String|Append "Rifle Ammo (" (Utilities|String|ToString(Integer) (Variables|Default|GetAmmoCount)) ")")))
      (Variables|Default|SetInUse false)
      (Default|SendUpdateAmmoPickup (.AsBR%20Game%20Mode (Utilities|Casting|CastToBR_GameMode (Game|GetGameMode))) (Variables|Default|GetInUse) (Variables|Default|GetAmmoCount) (Variables|Default|GetGUID))
      (else
        (Default|DeletefromGroundItems (.AsBR%20Game%20Mode (Utilities|Casting|CastToBR_GameMode (Game|GetGameMode))) self)))))

(fn ConstructionScript
  (Variables|Default|SetUseText (Utilities|Text|ToText(String) (Utilities|String|Append "Rifle Ammo (" (Utilities|String|ToString(Integer) (Variables|Default|GetAmmoCount)) ")")))
  (|CallParentFunction))