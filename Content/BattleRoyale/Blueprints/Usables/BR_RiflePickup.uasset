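; Rifle pickup usable for the Battle Royale mode that adds a rifle to the character who uses it.
; On use it sets an InUse lock sent through the game mode by GUID, then removes itself from ground items if AddWeapon succeeds, or releases the lock otherwise.
; ChangeWeapononID stores the weapon ID and sets mesh and use text, with a switch meant for rifle variants but only the base rifle set up.
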(event EventBeginPlay)

(event Collision|EventActorBeginOverlap
  (params (OtherActor :type Actor%20Object%20Reference)))

(event EventChangeWeapononID
  (params (WeaponID :type Integer))
  ;[1 1 1] Change Weapon On ID - Change Pickup Mesh and WeaponID
  (bind _output_get (Variables|Default|SetWeaponID WeaponID))
  ;;[0.2984 1 0.4245] Add more pins on switch based on ENUM_RiflePickupID to change into different rifles
  (switch int _output_get
    (:1
      ;;;[1 1 1] Base Mesh
      (Components|StaticMesh|SetStaticMesh (Variables|Default|GetStaticMeshComponent) "/Game/BattleRoyale/Meshes/AutoRifle/SM_Rifle.SM_Rifle")
      (Variables|Default|SetUseText "Rifle"))))

(event EventTick
  (params (DeltaSeconds :type Float%20%28single-precision%29)))

(event EventOnUsed
  (params (Character :type BR%20Character%20Object%20Reference))
  ;[1 1 1] OnUsed Override to Add Rifle Weapon to Character
  (if (not (Variables|Default|GetInUse))
    (bind _output_get (Variables|Default|SetInUse true))
    (Default|SendUpdatePickupinUse (.AsBR%20Game%20Mode (Utilities|Casting|CastToBR_GameMode (Game|GetGameMode))) _output_get (Variables|Default|GetGUID))
    (bind _success (Default|AddWeapon Character (Variables|Default|GetInventoryClass) (Variables|Default|GetWeaponID)))
    (if _success
      (Default|DeletefromGroundItems (.AsBR%20Game%20Mode (Utilities|Casting|CastToBR_GameMode (Game|GetGameMode))) self)
      (else
        (bind _output_get_2 (Variables|Default|SetInUse false))
        (Default|SendUpdatePickupinUse (.AsBR%20Game%20Mode (Utilities|Casting|CastToBR_GameMode (Game|GetGameMode))) _output_get_2 (Variables|Default|GetGUID))))))

(fn ConstructionScript
  (|CallParentFunction))