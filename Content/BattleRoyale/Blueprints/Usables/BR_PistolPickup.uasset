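; Battle royale pistol pickup that gives its weapon to the character who uses it.
; On use it sets an InUse lock, reports it through BR_GameMode, then calls AddWeapon.
; Success has the game mode delete it from ground items; failure releases and re-reports the lock.
; ChangeWeapononID stores the weapon ID and sets the mesh and use text, currently showing only the base 1911 pistol.
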(event EventBeginPlay)

(event Collision|EventActorBeginOverlap
  (params (OtherActor :type Actor%20Object%20Reference)))

(event EventTick
  (params (DeltaSeconds :type Float%20%28single-precision%29)))

(event EventChangeWeapononID
  (params (WeaponID :type Integer))
  ;[1 1 1] Change Weapon On ID - Change the Mesh of the pickup and the WeaponID
  (bind _output_get (Variables|Default|SetWeaponID WeaponID))
  ;;[0.205 1 0.5812] Add pins for each weapon in ENUM_PistolWeaponID
  (switch int _output_get
    (:1
      ;;;[1 1 1] Base Mesh
      (Components|StaticMesh|SetStaticMesh (Variables|Default|GetStaticMeshComponent) "/Game/BattleRoyale/Meshes/Pistol/SM_1911.SM_1911")
      (Variables|Default|SetUseText "Pistol"))))

(event EventOnUsed
  (params (Character :type BR%20Character%20Object%20Reference))
  ;[1 1 1] OnUsed Override to Add Pistol Weapon to Character
  (if (not (Variables|Default|GetInUse))
    (bind _output_get (Variables|Default|SetInUse true))
    (Default|SendUpdatePickupinUse (.AsBR%20Game%20Mode (Utilities|Casting|CastToBR_GameMode (Game|GetGameMode))) _output_get (Variables|Default|GetGUID))
    (bind _success (Default|AddWeapon Character (Variables|Default|GetInventoryClass) (Variables|Default|GetWeaponID)))
    (if _success
      (Default|DeletefromGroundItems (.AsBR%20Game%20Mode (Utilities|Casting|CastToBR_GameMode (Game|GetGameMode))) self)
      (else
        (bind _output_get_2 (Variables|Default|SetInUse false))
        (Default|SendUpdatePickupinUse (.AsBR%20Game%20Mode (Utilities|Casting|CastToBR_GameMode (Game|GetGameMode))) _output_get_2 (Variables|Default|GetGUID))))))

(fn ConstructionScript
  (|CallParentFunction))