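; Battle royale bandage pickup that adds its stack of bandages to the character who uses it.
; OnUsed locks the item with an InUse flag sent to multiplayer through BR_GameMode by GUID, then calls AddBandage on the character.
; An emptied pickup is deleted from ground items; otherwise any leftover count updates the use text and is sent out, and the lock is released.
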(event EventBeginPlay)

(event Collision|EventActorBeginOverlap
  (params (OtherActor :type Actor%20Object%20Reference)))

(event EventOnUsed
  (params (Character :type BR%20Character%20Object%20Reference))
  ;[1 1 1] OnUsed Override to add bandages to character - Send Multiplayer Functions when necessary
  ;;[0.003206 1 0.07555] Check if Item is not in use - if so then send update to set in use to true to multiplayer and add bandage to character
  (if (not (Variables|Default|GetInUse))
    (bind _output_get (Variables|Default|SetInUse true))
    (Default|SendUpdatePickupinUse (.AsBR%20Game%20Mode (Utilities|Casting|CastToBR_GameMode (Game|GetGameMode))) _output_get (Variables|Default|GetGUID))
    (bind (_success _bandagesleft) (Default|AddBandage Character (Variables|Default|GetCount)))
    (if _success
      (if (== _bandagesleft 0)
        ;;[0.04035 1 0.03873] All Bandages Taken - Delete from Ground
        (Default|DeletefromGroundItems (.AsBR%20Game%20Mode (Utilities|Casting|CastToBR_GameMode (Game|GetGameMode))) self)
        (else
          ;;[0.01768 1 0.08637] Not all bandages taken - set count of item, set use text, and send out multiplayer updates
          (Variables|Default|SetCount _bandagesleft)
          (Variables|Default|SetUseText (Utilities|Text|ToText(String) (Utilities|String|Append "Bandages (" (Utilities|String|ToString(Integer) (Variables|Default|GetCount)) ")")))
          (Default|SendUpdateBandagePickup (.AsBR%20Game%20Mode (Utilities|Casting|CastToBR_GameMode (Game|GetGameMode))) (Variables|Default|GetGUID) (Variables|Default|GetCount))
          (Variables|Default|SetInUse false)
          (Default|SendUpdatePickupinUse (.AsBR%20Game%20Mode (Utilities|Casting|CastToBR_GameMode (Game|GetGameMode))) false (Variables|Default|GetGUID))))
      (else
        ;;[0 1 0.1109] Not Successful when Adding Bandages to Character
        (Variables|Default|SetInUse false)
        (Default|SendUpdatePickupinUse (.AsBR%20Game%20Mode (Utilities|Casting|CastToBR_GameMode (Game|GetGameMode))) false (Variables|Default|GetGUID))))))

(event EventTick
  (params (DeltaSeconds :type Float%20%28single-precision%29)))

(fn ConstructionScript
  (Variables|Default|SetUseText (Utilities|Text|ToText(String) (Utilities|String|Append "Bandages (" (Utilities|String|ToString(Integer) (Variables|Default|GetCount)) ")")))
  (|CallParentFunction))