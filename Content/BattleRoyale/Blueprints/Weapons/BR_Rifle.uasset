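; Rifle weapon Blueprint for the Battle Royale mode, built as a child of a parent weapon class.
; BeginPlay and Reload defer to the parent, while Fire also increases hip-fire (non-ADS) spread by a fixed amount after the parent's logic.
; The ChangeWeapononID override stores the ID and switches on it to set the skeletal mesh, with only the base rifle mesh present so far.
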(event EventBeginPlay
  (|CallParentFunction))

(event Collision|EventActorBeginOverlap
  (params (OtherActor :type Actor%20Object%20Reference)))

(event EventChangeWeapononID
  (params (WeaponID :type Integer))
  ;[1 1 1] ChangeWeaponOnID override
  (bind _output_get (Variables|Default|SetWeaponID WeaponID))
  ;;[0.2433 1 0.2351] Add more pins to switch based on ENUM_RifleWeaponID
  (switch int _output_get
    (:1
      ;;;[1 1 1] Base Mesh
      (Class|SkinnedMeshComponent|SetSkeletalMesh (Variables|Default|GetWeaponMesh) "/Game/BattleRoyale/Meshes/AutoRifle/SKM_Rifle.SKM_Rifle" true))))

(event EventTick
  (params (DeltaSeconds :type Float%20%28single-precision%29)))

(event EventFire
  (|CallParentFunction)
  (CallFunction|IncreaseSpread 0.1 false))

(event EventReload
  (|CallParentFunction))

(fn ConstructionScript
  (|CallParentFunction))