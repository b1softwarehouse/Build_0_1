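; Base weapon for the battle royale game, handling hitscan fire, accuracy spread, reloading and montages, with a weapon-change stub for children.
; Fire traces from the camera within a spread cone that Tick eases toward the hip or ADS minimum.
; Hit surface type drives blood, delayed hit sounds and damage, including fixed headshot damage.
; Shots and ammo-bag reloads are sent through BR_GameMode, while GSFire plays multiplayer shots with third-person effects.
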(event Custom|Fire
  ;[1 1 1] Fire
  (CallFunction|PlayArmsFireMontage)
  (CallFunction|PlayWeaponFireMontage)
  (bind (_projectiletransform _hitresult _endlocation _peerid) (CallFunction|PerformFire))
  (Audio|PlaySoundatLocation (Variables|Default|GetFireSound) (.location (Transformation|GetWorldTransform (Default|GetCamera (Variables|Default|GetCharRef)))) "0, 0, 0" 0.5)
  (Effects|SpawnEmitterAttached (Variables|Default|GetMuzzleFX) (Variables|Default|GetWeaponMesh) (Variables|Default|GetMuzzleSocket) "0.0,0.0,0.0" "0.0,0.0,0.0")
  (bind _returnvalue (Effects|SpawnEmitteratLocation (Variables|Default|GetTrailFX) (Transformation|GetSocketLocation (Variables|Default|GetWeaponMesh) (Variables|Default|GetMuzzleSocket))))
  (Effects|Components|ParticleSystem|SetVectorParameter _returnvalue "ShockBeamEnd" _endlocation)
  (CallFunction|HitSound _hitresult)
  (bind _shouldspawnblood (CallFunction|SpawnBlood _hitresult _endlocation))
  (bind _newdamage (CallFunction|CalcDamage _hitresult))
  (Default|SendFire (.AsBR%20Game%20Mode (Utilities|Casting|CastToBR_GameMode (Game|GetGameMode))) _endlocation _shouldspawnblood _peerid _newdamage)
  (Math|Integer|DecrementInt (Variables|Default|GetCurrentAmmo)
    (:%20%20
      (Utilities|FlowControl|Delay 0.1)
      (Variables|/Game/BattleRoyale/Blueprints/BR_Character.BR_Character_C|SetIsFiring (Variables|Default|GetCharRef) false))))

(event Custom|StopReloadAnim
  ;[1 1 1] Stop Reload Animation Montage
  (bind _weaponreloadmontage (Variables|Default|GetWeaponReloadMontage)
    (:then
      (Animation|Montage|MontageStop (Components|SkeletalMesh|GetAnimInstance (Variables|Default|GetWeaponMesh)) 0.0 _weaponreloadmontage))
    (:else)))

(event Custom|ReloadAnim
  ;[1 1 1] Reload Animation Montage if Available
  (bind _weaponreloadmontage (Variables|Default|GetWeaponReloadMontage)
    (:then
      (Animation|Montage|MontagePlay (Components|SkeletalMesh|GetAnimInstance (Variables|Default|GetWeaponMesh)) _weaponreloadmontage 1.0 "MontageLength" 0.0))
    (:else)))

(event Custom|GSFire
  (params (EndLocation :type Vector) (ShouldSpawnBlood :type Boolean))
  ;[1 1 1] TPP Fire from Multiplayer
  (CallFunction|PlayTPPFireMontage)
  (CallFunction|PlayWeaponFireMontage)
  (Audio|PlaySoundatLocation (Variables|Default|GetFireSound) (Transformation|GetSocketLocation (Variables|Default|GetWeaponMesh) (Variables|Default|GetMuzzleSocket)))
  (Effects|SpawnEmitterAttached (Variables|Default|GetMuzzleFX) (Variables|Default|GetWeaponMesh) (Variables|Default|GetMuzzleSocket) "0.0,0.0,0.0" "0.0,0.0,0.0")
  (if ShouldSpawnBlood
    (bind _returnvalue (Effects|SpawnEmitteratLocation "/Game/BattleRoyale/Particles/P_body_bullet_impact.P_body_bullet_impact" EndLocation))
    (Transformation|SetRelativeScale3D _returnvalue "4.000000,4.000000,4.000000"))
  (Variables|/Game/BattleRoyale/Blueprints/BR_Character.BR_Character_C|SetIsFiring (Variables|Default|GetCharRef) false))

(event Custom|Reload
  ;[1 1 1] Reload
  (CallFunction|PerformReload))

(event EventBeginPlay
  ;[1 1 1] Event Begin Play
  (bind _asbr_character (Utilities|Casting|CastToBR_Character (Game|GetPlayerCharacter 0))
    (:then
      (Variables|Default|SetCharRef _asbr_character))
    (:CastFailed
      (Variables|Default|SetCharRef 0))))

(event Collision|EventActorBeginOverlap
  (params (OtherActor :type Actor%20Object%20Reference)))

(event EventTick
  (params (DeltaSeconds :type Float%20%28single-precision%29))
  ;[1 1 1] Change Accuracy Spread on Tick
  (Variables|Default|SetDeltaTime DeltaSeconds)
  (bind _charref (Variables|Default|GetCharRef)
    (:then
      (if (Variables|/Game/BattleRoyale/Blueprints/BR_Character.BR_Character_C|GetIsADS _charref)
        (if (>= (Variables|Default|GetSpreadCurrent) (Variables|Default|GetSpreadMinAim))
          (CallFunction|DecreaseSpread (* (Variables|Default|GetDeltaTime) (Variables|Default|GetSpreadDecreaseSpeed)) (Variables|/Game/BattleRoyale/Blueprints/BR_Character.BR_Character_C|GetIsADS (Variables|Default|GetCharRef)))
          (else
            (CallFunction|IncreaseSpreadtoMin (* (Variables|Default|GetDeltaTime) (Variables|Default|GetSpreadIncreaseSpeed)) (Variables|/Game/BattleRoyale/Blueprints/BR_Character.BR_Character_C|GetIsADS (Variables|Default|GetCharRef)))))
        (elif (>= (Variables|Default|GetSpreadCurrent) (Variables|Default|GetSpreadMinHip))
          (CallFunction|DecreaseSpread (* (Variables|Default|GetDeltaTime) (Variables|Default|GetSpreadDecreaseSpeed)) (Variables|/Game/BattleRoyale/Blueprints/BR_Character.BR_Character_C|GetIsADS (Variables|Default|GetCharRef)))
          (else
            (CallFunction|IncreaseSpreadtoMin (* (Variables|Default|GetDeltaTime) (Variables|Default|GetSpreadIncreaseSpeed)) (Variables|/Game/BattleRoyale/Blueprints/BR_Character.BR_Character_C|GetIsADS (Variables|Default|GetCharRef)))))))
    (:else)))

(fn ConstructionScript
  ;[1 1 1] If Spread is Disabled, set all spread values to 0 and they will never change
  (if (Variables|Default|GetDisableSpread)
    (Utilities|FlowControl|Sequence
      (:then_0
        (Variables|Default|SetSpreadMinAim 0.0))
      (:then_1
        (Variables|Default|SetSpreadMaxAim 0.0))
      (:then_2
        (Variables|Default|SetSpreadMinHip 0.0))
      (:then_3
        (Variables|Default|SetSpreadMaxHip 0.0))
      (:then_4
        (Variables|Default|SetSpreadCurrent 0.0)))))

(fn IncreaseSpread
  (params (IncreaseAmount :type Float%20%28single-precision%29) (IsADS :type Boolean))
  ;[1 1 1] Increase Spread by Set Amount
  (Utilities|FlowControl|Sequence
    (:then_0
      (if IsADS
        (LocalVariables|SetSpreadMax (Variables|Default|GetSpreadMaxAim))
        (else
          (LocalVariables|SetSpreadMax (Variables|Default|GetSpreadMaxHip)))))
    (:then_1
      (if (>= (+ IncreaseAmount (Variables|Default|GetSpreadCurrent)) (LocalVariables|GetSpreadMax))
        (Variables|Default|SetSpreadCurrent (LocalVariables|GetSpreadMax))
        (else
          (Variables|Default|SetSpreadCurrent (+ IncreaseAmount (Variables|Default|GetSpreadCurrent))))))))

(fn DecreaseSpread
  (params (DecreaseAmount :type Float%20%28single-precision%29) (IsADS :type Boolean))
  ;[1 1 1] Decrease Spread by Set Amount Dependent on ADS
  (Utilities|FlowControl|Sequence
    (:then_0
      (if IsADS
        (LocalVariables|SetSpreadMin (Variables|Default|GetSpreadMinAim))
        (else
          (LocalVariables|SetSpreadMin (Variables|Default|GetSpreadMinHip)))))
    (:then_1
      (if (<= (- (Variables|Default|GetSpreadCurrent) DecreaseAmount) (LocalVariables|GetSpreadMin))
        (Variables|Default|SetSpreadCurrent (LocalVariables|GetSpreadMin))
        (else
          (Variables|Default|SetSpreadCurrent (- (Variables|Default|GetSpreadCurrent) DecreaseAmount)))))))

(fn IncreaseSpreadtoMin
  (params (IncreaseAmount :type Float%20%28single-precision%29) (IsADS :type Boolean))
  ;[1 1 1] Increase Spread to Min - Useful when swapping to weapon with different min spread values
  (Utilities|FlowControl|Sequence
    (:then_0
      (if IsADS
        (LocalVariables|SetSpreadMax (Variables|Default|GetSpreadMinAim))
        (else
          (LocalVariables|SetSpreadMax (Variables|Default|GetSpreadMinHip)))))
    (:then_1
      (if (>= (+ IncreaseAmount (Variables|Default|GetSpreadCurrent)) (LocalVariables|GetSpreadMax))
        (Variables|Default|SetSpreadCurrent (LocalVariables|GetSpreadMax))
        (else
          (Variables|Default|SetSpreadCurrent (+ IncreaseAmount (Variables|Default|GetSpreadCurrent))))))))

(fn PerformFire
  (bind _charref (Variables|Default|GetCharRef))
  (bind _spreadcurrent (Variables|Default|GetSpreadCurrent))
  (bind _weaponmesh (Variables|Default|GetWeaponMesh))
  (bind _muzzlesocket (Variables|Default|GetMuzzleSocket))
  (bind _returnvalue (Transformation|GetSocketLocation _weaponmesh _muzzlesocket))
  (bind _camera (Default|GetCamera _charref))
  (bind _returnvalue_2 (* _spreadcurrent 0.5))
  (bind _returnvalue_3 (Transformation|GetWorldTransform _camera))
  (bind _returnvalue_4 (Math|Vector|GetForwardVector (.rotation _returnvalue_3)))
  (bind _returnvalue_5 (Class|KismetMathLibrary|RandomUnitVectorinCone _returnvalue_4 _returnvalue_2))
  (bind _returnvalue_6 (* _returnvalue_5 1e+04))
  (bind _returnvalue_7 (+ (.location _returnvalue_3) _returnvalue_6))
  ;[1 1 1] Perform The Line Trace for the Firing of the Weapon
  (Utilities|FlowControl|Sequence
    (:then_0
      (LocalVariables|SetLocalEndLocation _returnvalue_7)
      (bind (_outhit _returnvalue_8) (Collision|LineTraceByChannel (.location _returnvalue_3) _returnvalue_7 "TraceTypeQuery1" false (Utilities|Array|MakeArray (Variables|Default|GetCharRef)) "None"))
      (LocalVariables|SetLocalEndHitResult _outhit)
      (if _returnvalue_8
        (bind _asbr_character (Utilities|Casting|CastToBR_Character (.HitActor (Collision|BreakHitResult _outhit)))
          (:then
            (LocalVariables|SetLocalPeerId (Variables|/Game/BattleRoyale/Blueprints/BR_Character.BR_Character_C|GetId _asbr_character)))
          (:CastFailed
            _))
        (LocalVariables|SetLocalEndTransform (Math|Transform|MakeTransform _returnvalue (Math|Rotator|FindLookatRotation _returnvalue (.ImpactPoint (Collision|BreakHitResult _outhit)))))
        (LocalVariables|SetLocalEndLocation (.ImpactPoint (Collision|BreakHitResult _outhit)))
        (else
          (LocalVariables|SetLocalEndTransform (Math|Transform|MakeTransform _returnvalue (Pawn|GetControlRotation (.AsPawn (Utilities|Casting|CastToPawn (Components|GetOwner (Default|GetCamera (Variables|Default|GetCharRef))))) :!class /Script/Engine.Pawn))))))
    (:then_1
      (return (LocalVariables|GetLocalEndTransform) (LocalVariables|GetLocalEndHitResult) (LocalVariables|GetLocalEndLocation) (LocalVariables|GetLocalPeerId)))))

(fn HitSound
  (params (HitResult :type Hit%20Result%20Structure))
  (bind (_bblockinghit _binitialoverlap _time _location _impactpoint _normal _impactnormal _physmat) (Collision|BreakHitResult HitResult))
  ;[1 1 1] Play the Hit Sound Based on Physical Surface of Hit Target
  (if _bblockinghit
    (switch Utilities|FlowControl|Switch|SwitchonEPhysicalSurface (Variables|/Script/Engine.PhysicalMaterial|GetSurfaceType _physmat)
      (:SurfaceType1
        (Utilities|Time|SetTimerbyFunctionName 0 "PlayHeadshotSound" 0.3))
      (:SurfaceType2
        (Utilities|Time|SetTimerbyFunctionName 0 "PlayBodyshotSound" 0.2)))))

(fn PlayHeadshotSound
  ;[1 1 1] Play Headshot Sound
  (Audio|PlaySound2D "/Game/BattleRoyale/Audio/Cues/SC_Headshot.SC_Headshot"))

(fn PlayBodyshotSound
  ;[1 1 1] Play Bodyshot Sound
  (Audio|PlaySound2D "/Game/BattleRoyale/Audio/Cues/SC_Bodyshot.SC_Bodyshot"))

(fn SpawnBlood
  (params (HitResult :type Hit%20Result%20Structure) (Location :type Vector))
  (bind (_bblockinghit _binitialoverlap _time _location _impactpoint _normal _impactnormal _physmat) (Collision|BreakHitResult HitResult))
  ;[1 1 1] Spawn Blood Emitter Based on Hit Result at Input Location
  (if _bblockinghit
    (switch Utilities|FlowControl|Switch|SwitchonEPhysicalSurface (Variables|/Script/Engine.PhysicalMaterial|GetSurfaceType _physmat)
      (:SurfaceType_Default
        _)
      (:SurfaceType1
        (bind _returnvalue (Effects|SpawnEmitteratLocation "/Game/BattleRoyale/Particles/P_body_bullet_impact.P_body_bullet_impact" Location :!label _label))
        (Transformation|SetRelativeScale3D _returnvalue "4.000000,4.000000,4.000000")
        (return true))
      (:SurfaceType2
        (goto _label))
      (:SurfaceType3
        _)
      (:SurfaceType4
        _))
    (return false)))

(fn CalcDamage
  (params (HitResult :type Hit%20Result%20Structure))
  (bind (_bblockinghit _binitialoverlap _time _location _impactpoint _normal _impactnormal _physmat) (Collision|BreakHitResult HitResult))
  ;[1 1 1] Calculate Damage Based on Physical Material - Headshot always kills
  ;;[0 0.03133 1] 1.5.1 Fix: Only on Blocking Hit
  (if _bblockinghit
    (Utilities|FlowControl|Sequence
      (:then_0
        (switch Utilities|FlowControl|Switch|SwitchonEPhysicalSurface (Variables|/Script/Engine.PhysicalMaterial|GetSurfaceType _physmat)
          (:SurfaceType1
            (LocalVariables|SetLocalDamage 1.2e+02))
          (:SurfaceType2
            (LocalVariables|SetLocalDamage (Variables|Default|GetDamage)))))
      (:then_1
        (return (LocalVariables|GetLocalDamage))))))

(fn PerformReload
  (bind _returnvalue (Game|GetGameMode))
  (bind _charref (Variables|Default|GetCharRef))
  (bind _charref_2 (Variables|Default|GetCharRef))
  (bind _asbr_game_mode (Utilities|Casting|CastToBR_GameMode _returnvalue))
  (LocalVariables|SetLocalWeaponClass (Utilities|GetClass (Variables|/Game/BattleRoyale/Blueprints/BR_Character.BR_Character_C|GetCurrentWeapon _charref_2)))
  ;[1 1 1] Find Current Struct in Ammo Bag
  (bind (_array_element _array_index) (Utilities|Array|ForEachLoopwithBreak (Variables|/Game/BattleRoyale/Blueprints/BR_Character.BR_Character_C|GetAmmoBag _charref_2))
    (:LoopBody
      (if (== (.WeaponType (Utilities|Struct|BreakSTRUCT_Ammo _array_element)) (LocalVariables|GetLocalWeaponClass))
        (LocalVariables|SetLocalSTRUCTAmmo _array_element)
        (LocalVariables|SetLocalBagIndex _array_index)))
    (:Completed
      (if (< (- (.CurrentCount (Utilities|Struct|BreakSTRUCT_Ammo (LocalVariables|GetLocalSTRUCTAmmo))) (- (Variables|Default|GetMagSize) (Variables|Default|GetCurrentAmmo))) 0)
        ;[1 1 1] Not Enough Ammo in Bag to Reload Gun - set to 0 and add Current Count of Bag to Current Ammo
        (LocalVariables|SetLocalNewCurrentAmmo (+ (.CurrentCount (Utilities|Struct|BreakSTRUCT_Ammo (LocalVariables|GetLocalSTRUCTAmmo))) (Variables|Default|GetCurrentAmmo)))
        (bind _structout (Utilities|Struct|SetmembersinSTRUCT_Ammo (LocalVariables|GetLocalSTRUCTAmmo)))
        (Utilities|Array|SetArrayElem (Variables|/Game/BattleRoyale/Blueprints/BR_Character.BR_Character_C|GetAmmoBag (Variables|Default|GetCharRef)) (LocalVariables|GetLocalBagIndex) _structout)
        (else
          ;[1 1 1] Enough Ammo in Bag - Reduce count in Bag and set Current Ammo to Mag Size
          (bind _structout_2 (Utilities|Struct|SetmembersinSTRUCT_Ammo (LocalVariables|GetLocalSTRUCTAmmo) (- (.CurrentCount (Utilities|Struct|BreakSTRUCT_Ammo (LocalVariables|GetLocalSTRUCTAmmo))) (- (Variables|Default|GetMagSize) (Variables|Default|GetCurrentAmmo)))))
          (Utilities|Array|SetArrayElem (Variables|/Game/BattleRoyale/Blueprints/BR_Character.BR_Character_C|GetAmmoBag (Variables|Default|GetCharRef)) (LocalVariables|GetLocalBagIndex) _structout_2)
          (LocalVariables|SetLocalNewCurrentAmmo (Variables|Default|GetMagSize))))
      ;[1 1 1] Set Current Ammo and Send Multiplayer Updates
      (Variables|Default|SetCurrentAmmo (LocalVariables|GetLocalNewCurrentAmmo))
      (Default|SendUpdateAmmoBag _asbr_game_mode (Variables|/Game/BattleRoyale/Blueprints/BR_Character.BR_Character_C|GetAmmoBag _charref))
      (Default|SendUpdateWeaponAmmo _asbr_game_mode (Variables|/Game/BattleRoyale/Blueprints/BR_Character.BR_Character_C|GetSelectedWeaponIndex _charref) (Variables|Default|GetCurrentAmmo)))))

(fn ChangeWeapononID
  (params (WeaponID :type Integer))
  (Development|PrintString "This should be overridden!"))

(fn PlayArmsFireMontage
  (if (Variables|/Game/BattleRoyale/Blueprints/BR_Character.BR_Character_C|GetIsADS (Variables|Default|GetCharRef))
    (bind _fpparmsadsfiremontage (Variables|Default|GetFPPArmsADSFireMontage)
      (:then
        (Animation|Montage|MontagePlay (Components|SkeletalMesh|GetAnimInstance (Variables|/Game/BattleRoyale/Blueprints/BR_Character.BR_Character_C|GetFPP_Mesh (Variables|Default|GetCharRef))) _fpparmsadsfiremontage 1.0 "MontageLength" 0.0))
      (:else))
    (else
      (bind _fpparmsfiremontage (Variables|Default|GetFPPArmsFireMontage)
        (:then
          (Animation|Montage|MontagePlay (Components|SkeletalMesh|GetAnimInstance (Variables|/Game/BattleRoyale/Blueprints/BR_Character.BR_Character_C|GetFPP_Mesh (Variables|Default|GetCharRef))) _fpparmsfiremontage 1.0 "MontageLength" 0.0))
        (:else)))))

(fn PlayWeaponFireMontage
  (bind _weaponfiremontage (Variables|Default|GetWeaponFireMontage)
    (:then
      (Animation|Montage|MontagePlay (Components|SkeletalMesh|GetAnimInstance (Variables|Default|GetWeaponMesh)) _weaponfiremontage 1.0 "MontageLength" 0.0))
    (:else)))

(fn PlayTPPFireMontage
  (bind _tppfiremontage (Variables|Default|GetTPPFireMontage)
    (:then
      (Animation|Montage|MontagePlay (Components|SkeletalMesh|GetAnimInstance (Variables|/Script/Engine.Character|GetMesh (Variables|Default|GetCharRef))) _tppfiremontage 1.0 "MontageLength" 0.0))
    (:else)))