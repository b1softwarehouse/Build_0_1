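; BR_GameInstance is the battle royale game instance that relays GameSparks connection, login, logout and matchmaking events between menus and game logic.
; Each custom event just fires a matching event dispatcher, passing credentials for authentication and clearing IsCurrentlyMatching when a match is found.
; On Init it picks the match short code from AllowTPP, keeping third-person and first-person players in separate matches.
; Shutdown fires a dispatcher to disconnect from GameSparks.
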(event Custom|GSMatchNotFound
  ;[1 1 1] MatchNotFound - call dispatcher to update test and button in UILobby
  (Default|CallGSMatchNotFoundDispatcher))

(event Custom|GSLogout
  ;[1 1 1] Call Logout Dispatcher to logout of GS
  (Default|CallGSLogoutDispatcher))

(event Custom|InitialGSConnect
  ;[1 1 1] Call InitialConnect dispatcher to show login box
  (Default|CallInitialGSConnectDispatcher))

(event Custom|GSCancelMatchmaking
  ;[1 1 1] GSCancelMatchmaking - call cancel matchmaking dispatcher to change Lobby text and button
  (Default|CallGSCancelMMDispatcher))

(event Custom|GSMatchmake
  ;[1 1 1] GSMatchmake - call matchmake dispatcher to start finding a match
  (Default|CallGSMatchmakeDispatcher))

(event Custom|GSAvailable
  ;[1 1 1] Gamesparks is available - call dispatcher to show login box
  (Default|CallGSAvailableDispatcher))

(event Custom|GSAuthSuccess
  ;[1 1 1] GSAuthSuccess - call auth success dispatcher to login to lobby
  (Default|CallGSAuthSuccessDispatcher))

(event Custom|GSAuthFailure
  ;[1 1 1] GSAuthFailure - call AuthFailure dispatcher to show login failed
  (Default|CallGSAuthFailureDispatcher))

(event Custom|GSAuthenticateUser
  (params (UserName :type Text) (Password :type Text))
  ;[1 1 1] Call AuthenticateUser dispatcher for MenuGameMode to login and go from Login to Lobby
  (Default|CallGSAuthenticateUserDispatcher UserName Password))

(event Custom|GSMatchFound
  ;[1 1 1] MatchFound - set IsCurrentlyMatching and call dispatcher to change to Arena level
  (Variables|Default|SetIsCurrentlyMatching false)
  (Default|CallGSMatchFoundDispatcher))

(event EventShutdown
  ;[1 1 1] Shutdown - call dispatcher to DC from Gamesparks
  (Default|CallGIShutdown))

(event EventInit
  ;[1 1 1] If AllowTPP is on, we want to change the short code so FPP players aren't in the same game
  (if (Variables|Default|GetAllowTPP)
    (Variables|Default|SetCurrentMatchShortCode (Utilities|String|EnumtoString (Utilities|Enum|LiteralenumENUM_MatchShortCodes "NewEnumerator5")))
    (else
      (Variables|Default|SetCurrentMatchShortCode (Utilities|String|EnumtoString (Utilities|Enum|LiteralenumENUM_MatchShortCodes "NewEnumerator4"))))))